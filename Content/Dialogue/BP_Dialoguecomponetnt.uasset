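; Dialogue component that runs data-table-driven conversations in a WB_Dialogue widget.
; Interact opens the widget with mouse input or advances it, as each row supplies the next row, table and end flag for closing.
; Branching options spawn as WB_Option widgets only when dialogue opens.
; Optionselected clears them and shows the chosen row, but stores the next row in Name, whereas Interact reads RowName.
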(event Custom|Option%20selected
  (params (RowName :type Name) (DataTable :type Data%20Table%20Object%20Reference))
  (bind _dialoguewidget (Variables|Default|GetDialoguewidget))
  (bind _returnvalue (Utilities|GetDataTableRow DataTable RowName)
    (:then
      (Widget|Panel|ClearChildren (Variables|/Game/Dialogue/WB_Dialogue.WB_Dialogue_C|Getoptionscrollbox _dialoguewidget))
      (Default|UpdateDialogue _dialoguewidget (.Dialogue (Utilities|Struct|BreakDialogue_Structure _returnvalue)))
      (Variables|Default|SetName (.Row (Utilities|Struct|BreakDialogue_Structure _returnvalue)))
      (Variables|Default|SetData%20Table (.Datatable (Utilities|Struct|BreakDialogue_Structure _returnvalue)))
      (Variables|Default|SetEnddialogue (.EndDialogue? (Utilities|Struct|BreakDialogue_Structure _returnvalue))))))

(event EventBeginPlay)

(event EventTick
  (params (DeltaSeconds :type Float%20%28single-precision%29)))

(event EventInteract
  (params (Player :type Gracz%20Object%20Reference))
  (bind _returnvalue (Game|GetPlayerController 0))
  (bind _returnvalue_2 (Game|GetPlayerController 0))
  (if (Variables|Default|GetEnddialogue)
    (Widget|RemovefromParent (Variables|Default|GetDialoguewidget))
    (Variables|Default|SetEnddialogue false)
    (Variables|Default|SetDialoguewidget 0)
    (Input|SetInputModeGameOnly _returnvalue false)
    (Variables|/Script/Engine.PlayerController|SetbShowMouseCursor _returnvalue false)
    (else
      (Utilities|IsValid (Variables|Default|GetDialoguewidget)
        (:Is%20Valid
          (bind _returnvalue_3 (Utilities|GetDataTableRow (Variables|Default|GetData%20Table) (Variables|Default|GetRow%20Name))
            (:then
              (Default|UpdateDialogue (Variables|Default|GetDialoguewidget) (.Dialogue (Utilities|Struct|BreakDialogue_Structure _returnvalue_3)))
              (Variables|Default|SetRow%20Name (.Row (Utilities|Struct|BreakDialogue_Structure _returnvalue_3)))
              (Variables|Default|SetData%20Table (.Datatable (Utilities|Struct|BreakDialogue_Structure _returnvalue_3)))
              (Variables|Default|SetEnddialogue (.EndDialogue? (Utilities|Struct|BreakDialogue_Structure _returnvalue_3))))))
        (:Is%20Not%20Valid
          (bind _returnvalue_4 (Utilities|GetDataTableRow (Variables|Default|GetData%20Table) (Variables|Default|GetRow%20Name))
            (:then
              (bind _returnvalue_5 (UserInterface|CreateWidget "/Game/Dialogue/WB_Dialogue.WB_Dialogue_C" 0 (Utilities|Text|ToText(Name) (Variables|Default|GetName)) (.Dialogue (Utilities|Struct|BreakDialogue_Structure _returnvalue_4))))
              (bind _output_get (Variables|Default|SetDialoguewidget _returnvalue_5))
              (UserInterface|Viewport|AddtoViewport _output_get 0)
              (Variables|Default|SetRow%20Name (.Row (Utilities|Struct|BreakDialogue_Structure _returnvalue_4)))
              (Variables|Default|SetData%20Table (.Datatable (Utilities|Struct|BreakDialogue_Structure _returnvalue_4)))
              (Variables|Default|SetEnddialogue (.EndDialogue? (Utilities|Struct|BreakDialogue_Structure _returnvalue_4)))
              (Input|SetInputModeGameandUI _returnvalue_2 0 "DoNotLock" true false)
              (Variables|/Script/Engine.PlayerController|SetbShowMouseCursor _returnvalue_2 true)
              (if (.Openededdialogue? (Utilities|Struct|BreakDialogue_Structure _returnvalue_4))
                (for _array_element (.Openendeddialogue? (Utilities|Struct|BreakDialogue_Structure _returnvalue_4))
                  (bind _returnvalue_6 (UserInterface|CreateWidget "/Game/Dialogue/WB_Option.WB_Option_C" 0 (Utilities|Text|ToText(Name) (.Optionalname (Utilities|Struct|BreakOptionsdialogue_Structure _array_element))) self (.Row (Utilities|Struct|BreakOptionsdialogue_Structure _array_element)) (.Datatable (Utilities|Struct|BreakOptionsdialogue_Structure _array_element))))
                  (Widget|Panel|AddChild (Variables|/Game/Dialogue/WB_Dialogue.WB_Dialogue_C|Getoptionscrollbox (Variables|Default|GetDialoguewidget)) _returnvalue_6))))))))))

(event EventLeaveDialogue
  (bind _returnvalue (Game|GetPlayerController 0))
  (Utilities|IsValid (Variables|Default|GetDialoguewidget)
    (:Is%20Valid
      (Widget|RemovefromParent (Variables|Default|GetDialoguewidget))
      (Variables|Default|SetEnddialogue false)
      (Variables|Default|SetDialoguewidget 0)
      (Input|SetInputModeGameOnly _returnvalue false)
      (Variables|/Script/Engine.PlayerController|SetbShowMouseCursor _returnvalue false))))