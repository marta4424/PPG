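; BP_Trader is a trader NPC with a shop screen and an overhead health bar.
; OpenShop creates the BW_Sklep widget as KupPrzWidget, showing the cursor with game-and-UI input.
; CloseShop restores game-only input but removes a differently named variable, BwSklep.
; Each Tick writes Zdrowie (health) into the NPC_Zdrowie widget's bar and rotates that widget component to face the player camera.
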(event Custom|OpenShop
  (bind _returnvalue (Game|GetPlayerController 0))
  (bind _returnvalue_2 (UserInterface|CreateWidget "/Game/UI/BW_Sklep.BW_Sklep_C"))
  (bind _output_get (Variables|Default|SetKupPrzWidget _returnvalue_2))
  (UserInterface|Viewport|AddtoViewport _output_get 0)
  (Variables|/Script/Engine.PlayerController|SetbShowMouseCursor _returnvalue true)
  (Input|SetInputModeGameandUI _returnvalue (Variables|Default|GetKupPrzWidget) "DoNotLock" true false))

(event Custom|CloseShop
  (bind _returnvalue (Game|GetPlayerController 0))
  (Widget|RemovefromParent (Variables|Default|Getbw_sklep))
  (Variables|/Script/Engine.PlayerController|SetbShowMouseCursor _returnvalue false)
  (Input|SetInputModeGameOnly _returnvalue false))

(event EventTick
  (params (DeltaSeconds :type Float%20%28single-precision%29))
  (bind _zdrowiepasek (Variables|Default|GetZdrowiePasek))
  (bind _asnpc_zdrowie (Utilities|Casting|CastToNPC_Zdrowie (UserInterface|GetWidget (Variables|Default|GetZdrowiePasek))))
  (Progress|SetPercent (Variables|/Game/UI/NPC_Zdrowie.NPC_Zdrowie_C|GetZdrowieNPC _asnpc_zdrowie) (/ (Variables|Default|Getzdrowie) 1e+02))
  (Transformation|SetWorldRotation _zdrowiepasek (Math|Rotator|FindLookatRotation (Transformation|GetWorldLocation _zdrowiepasek) (Transformation|GetWorldLocation (Variables|/Script/Engine.PlayerCameraManager|GetTransformComponent (Game|GetPlayerCameraManager 0)))) false false))

(fn ConstructionScript)