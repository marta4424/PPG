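; Inventory ("Ekwipunek") Blueprint that sets up an item array and toggles the inventory screen.
; On BeginPlay it creates and stores the WB_Ekwipunek widget and resizes the Items array to a fixed slot count.
; The I key adds the widget to the viewport or removes it, depending on its visibility.
; A LoadInventory call that passes this object to the widget is unwired and never runs.
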(event EventBeginPlay
  (bind _returnvalue (UserInterface|CreateWidget "/Game/Ekwipunek/Widgets/WB_Ekwipunek.WB_Ekwipunek_C"))
  (Variables|Default|SetEkwipunekWD _returnvalue)
  (Utilities|Array|Resize (Variables|Default|GetItems) 10))

(event EventTick
  (params (DeltaSeconds :type Float%20%28single-precision%29)))

(event Input|KeyboardEvents|I
  (params (Key :type Key%20Structure :default "None"))
  (bind _ekwipunekwd (Variables|Default|GetEkwipunekWD))
  (:Pressed
    (if (Widget|IsVisible (Variables|Default|GetEkwipunekWD))
      (Widget|RemovefromParent _ekwipunekwd)
      (else
        (UserInterface|Viewport|AddtoViewport _ekwipunekwd 0)))))